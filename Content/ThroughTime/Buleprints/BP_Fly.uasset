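; BP_Fly is a player-controlled flying pawn that moves constantly forward each tick with a swept location update.
; Enhanced Input drives looking, right/up movement, and speed changes through an acceleration curve, clamped to factors of the normal speed.
; When speed input is released, the speed returns to normal via FInterpTo.
; Tick also draws a debug camera-forward trace whose result is unused, and a Teleport function relocates the pawn.
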(event `self.ReceiveBeginPlay`
  (set `self.CurrentSpeed` (`self.NormalSpeed`))
  (`EnhancedInputSubsystemInterface.AddMappingContext` (pcsubsystem `EnhancedInputLocalPlayerSubsystem` (`GameplayStatics.GetPlayerController` 0)) "/Game/ThroughTime/Buleprints/Input/IMC_Fly.IMC_Fly" 0 (struct)))

(event `self.ReceiveTick`
  (params (DeltaSeconds :type "Float (single-precision)"))
  (bind _returnvalue (`self.K2_GetActorLocation`))
  (if (not (`self.ControlSpeed?`))
    (set `self.CurrentSpeed` (`KismetMathLibrary.FInterpTo` (`self.CurrentSpeed`) (`self.NormalSpeed`) 1.0)))
  (`self.K2_SetActorLocation` (+ (* (`self.GetActorForwardVector`) (* DeltaSeconds (`self.CurrentSpeed`))) (`self.K2_GetActorLocation`)) true)
  (`KismetSystemLibrary.LineTraceSingle` :`Start` _returnvalue :`End` (+ _returnvalue (* (`SceneComponent.GetForwardVector` (`self.Camera`)) 20000.0)) :`TraceChannel` "TraceTypeQuery1" :`DrawDebugType` "ForOneFrame"))

(event `EnhancedInput|/Game/FirstPerson/Input/Actions/IA_Look`
  (params (ActionValue :type "Vector2D Structure") (ElapsedSeconds :type "Float (double-precision)") (TriggeredSeconds :type "Float (double-precision)") (InputAction :type "InputAction Object Reference" :default "/Game/FirstPerson/Input/Actions/IA_Look.IA_Look"))
  (:`Triggered`
    (`self.AddControllerYawInput` ActionValue_X)
    (`self.AddControllerPitchInput` ActionValue_Y)))

(event `EnhancedInput|/Game/FirstPerson/Input/Actions/IA_Move`
  (params (ActionValue :type "Vector2D Structure") (ElapsedSeconds :type "Float (double-precision)") (TriggeredSeconds :type "Float (double-precision)") (InputAction :type "InputAction Object Reference" :default "/Game/FirstPerson/Input/Actions/IA_Move.IA_Move"))
  (:`Triggered`
    (`self.AddMovementInput` (`self.GetActorRightVector`) ActionValue_X)
    (`self.AddMovementInput` (`self.GetActorUpVector`) ActionValue_Y)))

(event `EnhancedInput|/Game/ThroughTime/Buleprints/Input/IA_Speed`
  (params (ActionValue :type "Float (double-precision)") (ElapsedSeconds :type "Float (double-precision)") (TriggeredSeconds :type "Float (double-precision)") (InputAction :type "InputAction Object Reference" :default "/Game/ThroughTime/Buleprints/Input/IA_Speed.IA_Speed"))
  (bind _normalspeed (`self.NormalSpeed`))
  (:`Triggered`
    (set `self.CurrentSpeed` (`KismetMathLibrary.FClamp` (+ (`self.CurrentSpeed`) (`CurveFloat.GetFloatValue` (`self.AccelerationCurve`) ActionValue)) (* (`self.MinSpeedFactor`) _normalspeed) (* _normalspeed (`self.MaxSpeedFactor`)))))
  (:`Started`
    (set `self.ControlSpeed?` true))
  (:`Canceled`
    (set `self.ControlSpeed?` false :!label _label))
  (:`Completed`
    (goto _label)))

(fn `Teleport`
  (params (TargetLocation :type "Vector Structure"))
  (`self.K2_SetActorLocation` TargetLocation false true))

(fn `UserConstructionScript`)