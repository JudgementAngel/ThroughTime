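; BP_EnemySpline is a spline path actor that spawns an enemy and hands it the route to move along.
; SetSplinePoint builds the path in world space, appending a point when the index is out of range, then setting its location and rotation.
; BeginMove spawns BP_Enemy at the last point, passes it this spline and scales its Timeline play rate to the inverse of AllTime.
; GetNextPoint is an empty stub.
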(event `self.ReceiveBeginPlay`)

(event `self.ReceiveTick`
  (params (DeltaSeconds :type "Float (single-precision)")))

(fn `BeginMove`
  (params (AllTime :type "Float (double-precision)" :default 10.0))
  (bind _spline (`self.Spline`))
  (bind _returnvalue (- (`SplineComponent.GetNumberOfSplinePoints` _spline) 1))
  (bind _returnvalue_2 (`|SpawnActorFromClass` "/Game/ThroughTime/Buleprints/BP_Enemy.BP_Enemy_C" (`KismetMathLibrary.MakeTransform` (`SplineComponent.GetLocationAtSplinePoint` _spline _returnvalue "World") (`SplineComponent.GetRotationAtSplinePoint` _spline _returnvalue "World")) "Undefined" "MultiplyWithRoot" null null))
  (bind _output_get (set `self.EnemyActor` _returnvalue_2))
  (set `/Game/ThroughTime/Buleprints/BP_Enemy.EnemySpline` self _output_get)
  (bind _output_get_2 (set `/Game/ThroughTime/Buleprints/BP_Enemy.AllTime` AllTime _output_get))
  (`TimelineComponent.SetPlayRate` (`/Game/ThroughTime/Buleprints/BP_Enemy.Timeline` _output_get) (/ 1.0 _output_get_2)))

(fn `GetNextPoint`)

(fn `SetSplinePoint`
  (params (PointIndex :type Integer) (Location :type "Vector Structure") (Rotation :type "Rotator Structure"))
  (bind _spline (`self.Spline`))
  (bind _spline_2 (`self.Spline`))
  (bind _returnvalue (`SplineComponent.GetNumberOfSplinePoints` _spline_2))
  (if (>= PointIndex _returnvalue)
    (`SplineComponent.AddSplinePointAtIndex` _spline_2 Location _returnvalue "World" true))
  (`SplineComponent.SetLocationAtSplinePoint` _spline (`local.PointIndex`) Location "World" true)
  (`SplineComponent.SetRotationAtSplinePoint` _spline (`local.PointIndex`) Rotation "World" true))

(fn `UserConstructionScript`)