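; BP_Enemy is a hazard actor that randomly becomes a Speed or Distance enemy on BeginPlay, with a matching material.
; After a short arming delay, overlaps branch on type: projectile hits destroy only Speed enemies and boost the shooter's normal speed.
; Touching BP_Fly ends the game for Speed enemies or decreases distance for Distance enemies, then destroys the enemy.
; Timeline-driven spline movement is present but unconnected.
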(event `self.ReceiveBeginPlay`
  (`|ExecutionSequence`
    (:`then_0`
      (if (`KismetMathLibrary.RandomBool`)
        (set `self.EnemyType` "NewEnumerator1")
        (`PrimitiveComponent.SetMaterial` (`self.FlyChar`) 0 (`self.DistanceEnemyMaterial`))
        (else
          (set `self.EnemyType` "NewEnumerator0")
          (`PrimitiveComponent.SetMaterial` (`self.FlyChar`) 0 (`self.SpeedEnemyMaterial`)))))
    (:`then_1`
      (`KismetSystemLibrary.Delay` 0.2)
      (set `self.CanOverlap?` true))))

(event `self.ReceiveActorBeginOverlap`
  (params (OtherActor :type "Actor Object Reference"))
  (if (`self.CanOverlap?`)
    (bind _asbp_fly_person_projectile (cast `/Game/ThroughTime/Buleprints/BP_FlyPersonProjectile` OtherActor)
      (:`then`
        (switch `/Game/ThroughTime/Buleprints/E_EnemyType` (`self.EnemyType`)
          (:`NewEnumerator0`
            (`/Game/ThroughTime/Buleprints/BP_Fly.IncreaseNormalSpeed` (`/Game/ThroughTime/Buleprints/BP_FlyPersonProjectile.FlyOwner` _asbp_fly_person_projectile) 200.0)
            (`self.K2_DestroyActor` _asbp_fly_person_projectile))))
      (:`CastFailed`
        (bind _asbp_fly (cast `/Game/ThroughTime/Buleprints/BP_Fly` OtherActor))
        (switch `/Game/ThroughTime/Buleprints/E_EnemyType` (`self.EnemyType`)
          (:`NewEnumerator0`
            (message `/Game/ThroughTime/Buleprints/BPI_GameLife.GameEnd` _asbp_fly))
          (:`NewEnumerator1`
            (`/Game/ThroughTime/Buleprints/BP_Fly.DecreaseDistance` _asbp_fly)))))
    (`self.K2_DestroyActor`)))

(fn `UserConstructionScript`)