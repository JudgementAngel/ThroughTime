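; BP_TriggerBox is a trigger actor that teleports a BP_Fly back to a transport point when it overlaps the end box.
; The destination is the actor location plus TransportPoint, with random Y and Z offsets drawn from the RandomPlane ranges.
; The construction script moves the transport plane and begin box to TransportPoint.
; The begin box overlap only casts to BP_Fly and does nothing further.
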(event `self.End_Box.OnComponentBeginOverlap`
  (params (OverlappedComponent :type "PrimitiveComponent Object Reference") (OtherActor :type "Actor Object Reference") (OtherComp :type "PrimitiveComponent Object Reference") (OtherBodyIndex :type Integer) (bFromSweep :type Boolean) (SweepResult :type "HitResult Structure (by ref)"))
  (bind (_randomplane_x _randomplane_y _randomplane_z _randomplane_w) (`KismetMathLibrary.BreakVector4` (`self.RandomPlane`)))
  (bind _asbp_fly (cast `/Game/ThroughTime/Buleprints/BP_Fly` OtherActor))
  (`/Game/ThroughTime/Buleprints/BP_Fly.Teleport` _asbp_fly (+ (`self.K2_GetActorLocation`) (`self.TransportPoint`) (`KismetMathLibrary.MakeVector` 0.0 (`KismetMathLibrary.RandomFloatInRange` _randomplane_x _randomplane_y) (`KismetMathLibrary.RandomFloatInRange` _randomplane_z _randomplane_w)))))

(event `self.Begin_Box.OnComponentBeginOverlap`
  (params (OverlappedComponent :type "PrimitiveComponent Object Reference") (OtherActor :type "Actor Object Reference") (OtherComp :type "PrimitiveComponent Object Reference") (OtherBodyIndex :type Integer) (bFromSweep :type Boolean) (SweepResult :type "HitResult Structure (by ref)"))
  (cast `/Game/ThroughTime/Buleprints/BP_Fly` OtherActor))

(fn `UserConstructionScript`
  (bind _transportpoint (`self.TransportPoint`))
  (`SceneComponent.K2_SetRelativeLocation` (`self.TransportPlane`) _transportpoint false false)
  (`SceneComponent.K2_SetRelativeLocation` (`self.Begin_Box`) _transportpoint false false))